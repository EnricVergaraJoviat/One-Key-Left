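; BP_PlatformCountdown1 is a moving platform that starts a countdown to collapse when something overlaps its trigger box.
; BeginPlay puts a dynamic emissive material on StaticMesh1, and Tick shifts its ColorLerp parameter as the timer runs down from TimeToDestroy.
; At zero it destroys the box, spline and InterpToMovement components, then enables physics simulation on StaticMesh so the platform falls.
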(event `self.ReceiveBeginPlay`
  (`parent.ReceiveBeginPlay`)
  (bind _returnvalue (`KismetMaterialLibrary.CreateDynamicMaterialInstance` "/Game/Platformer_8_Underworld/Materials/M_emissio_2.M_emissio_2"))
  (bind _output_get (set `self.DynamicMat` _returnvalue))
  (`PrimitiveComponent.SetMaterial` (`self.StaticMesh1`) 0 _output_get)
  (set `self.timer` (`self.timeToDestroy`)))

(event `self.ReceiveTick`
  (params (DeltaSeconds :type "Float (single-precision)"))
  (`parent.ReceiveTick` DeltaSeconds)
  (if (`self.StartCountdown`)
    (bind _output_get (set `self.timer` (- (`self.timer`) DeltaSeconds)))
    (`MaterialInstanceDynamic.SetScalarParameterValue` (`self.DynamicMat`) "ColorLerp" (- 1.0 (/ (`self.timer`) (`self.timeToDestroy`))))
    (if (< _output_get 0.0)
      (set `self.StartCountdown` false)
      (`ActorComponent.K2_DestroyComponent` (`self.Box`))
      (`ActorComponent.K2_DestroyComponent` (`self.Spline`))
      (`ActorComponent.K2_DestroyComponent` (`self.InterpToMovement`))
      (`PrimitiveComponent.SetSimulatePhysics` (`self.StaticMesh`) true))))

(event `self.Box.OnComponentBeginOverlap`
  (params (OverlappedComponent :type "PrimitiveComponent Object Reference") (OtherActor :type "Actor Object Reference") (OtherComp :type "PrimitiveComponent Object Reference") (OtherBodyIndex :type Integer) (bFromSweep :type Boolean) (SweepResult :type "HitResult Structure (by ref)"))
  (set `self.StartCountdown` true))

(fn `UserConstructionScript`
  (`parent.UserConstructionScript`))