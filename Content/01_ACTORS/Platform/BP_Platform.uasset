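; BP_Platform is a moving platform whose path is authored with a spline.
; On BeginPlay it copies each spline point into InterpToMovement as a relative control point and applies Duration, so movement interpolates between points rather than following the spline's curves.
; When PreviewInEditor is enabled, the Construction Script places the static mesh along the spline by PreviewAlpha, a fraction of the spline's length.
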(event `self.ReceiveBeginPlay`
  (set `self.PreviewInEditor` false)
  (set `InterpToMovementComponent.Duration` (`self.Duration`) (`self.InterpToMovement`))
  (for _index (range (`SplineComponent.GetNumberOfSplinePoints` (`self.Spline`)))
    (`InterpToMovementComponent.AddControlPointPosition` (`self.InterpToMovement`) (`SplineComponent.GetLocationAtSplinePoint` (`self.Spline`) _index "Local") true))
  (`InterpToMovementComponent.FinaliseControlPoints` (`self.InterpToMovement`)))

(fn `UserConstructionScript`
  (if (`self.PreviewInEditor`)
    (`SceneComponent.K2_SetRelativeLocation` (`self.StaticMesh`) (`SplineComponent.GetLocationAtDistanceAlongSpline` (`self.Spline`) (* (`SplineComponent.GetSplineLength` (`self.Spline`)) (`self.PreviewAlpha`)) "Local") false false)))