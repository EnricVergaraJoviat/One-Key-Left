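; BP_FinalDoor is a final door that opens only when the player has collected all keys.
; OpenDoor casts the player character to BP_FirstPersonCharacter and checks AreAllKeysCollected.
; On success it plays an opening sound, calls OpenDoorAnimation (not defined here) and sets Opened to prevent repeats, returning true.
; With keys missing it plays an error sound and returns false.
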(fn `OpenDoor`
  (returns (opened :type Boolean))
  (bind _asbp_first_person_character (cast `/Game/FirstPerson/Blueprints/BP_FirstPersonCharacter` (`GameplayStatics.GetPlayerCharacter` 0)))
  (bind _allcollected (`/Game/FirstPerson/Blueprints/BP_FirstPersonCharacter.AreAllKeysCollected` _asbp_first_person_character))
  (if _allcollected
    (if (not (`self.Opened`))
      (`GameplayStatics.PlaySound2D` "/Game/02_Sounds/Door-opening_modified.Door-opening_modified" 1.0 1.0 0.0 null null)
      (`self.OpenDoor_Animation`)
      (set `self.Opened` true)
      (return true))
    (else
      (`GameplayStatics.PlaySound2D` "/Game/02_Sounds/Error.Error" 1.0 1.0 0.0 null null)
      (return false))))

(fn `UserConstructionScript`
  (`parent.UserConstructionScript`))