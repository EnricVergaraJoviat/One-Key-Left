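; BP_Door is a double sliding door actor whose two panels slide apart along world X.
; BeginPlay caches each panel's world position and a fixed opposite offset as its open position.
; The OpenDoor_Animation event plays a timeline that lerps both panels toward those positions, with no closing logic.
; The separate OpenDoor function is a stub returning false, and nothing in this Blueprint calls the animation event.
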(event `self.ReceiveBeginPlay`
  (set `self.InitialPos_Right` (`SceneComponent.K2_GetComponentLocation` (`self.door_right`)))
  (set `self.InitialPos_Left` (`SceneComponent.K2_GetComponentLocation` (`self.door_left`)))
  (set `self.FinalPos_Right` (+ (`self.InitialPos_Right`) (200.0 0.0 0.0)))
  (set `self.FinalPos_Left` (+ (`self.InitialPos_Left`) (-200.0 0.0 0.0))))

(event `OpenDoor_Animation`
  (bind (_direction _newtrack_0) (`Timeline|Timeline`)
    (:`Update`
      (`SceneComponent.K2_SetWorldLocation` (`self.door_right`) (`KismetMathLibrary.VLerp` (`self.InitialPos_Right`) (`self.FinalPos_Right`) _newtrack_0) false false)
      (`SceneComponent.K2_SetWorldLocation` (`self.door_left`) (`KismetMathLibrary.VLerp` (`self.InitialPos_Left`) (`self.FinalPos_Left`) _newtrack_0) false false))))

(fn `OpenDoor`
  (returns (opened :type Boolean))
  (return false))

(fn `UserConstructionScript`)