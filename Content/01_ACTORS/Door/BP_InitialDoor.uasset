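; BP_InitialDoor is a door that starts a countdown when first opened, killing the player if time runs out.
; OpenDoor runs once: it plays a sound and the opening animation, then shows the player's UI with the collected and total key counts.
; Tick then decrements the timer, updates the countdown display and calls Die on the cached first-person character once it drops below zero.
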(event `self.ReceiveBeginPlay`
  (`parent.ReceiveBeginPlay`)
  (bind _asbp_first_person_character (cast `/Game/FirstPerson/Blueprints/BP_FirstPersonCharacter` (`GameplayStatics.GetPlayerCharacter` 0)))
  (set `self.Player` _asbp_first_person_character))

(event `self.ReceiveTick`
  (params (DeltaSeconds :type "Float (single-precision)"))
  (`parent.ReceiveTick` DeltaSeconds)
  (if (`self.StartCountdown`)
    (bind _output_get (set `self.TimerCountdown` (- (`self.TimerCountdown`) DeltaSeconds)))
    (`/Game/FirstPerson/Player_UI.UpdateCountdown` (`/Game/FirstPerson/Blueprints/BP_FirstPersonCharacter.PlayerUI` (`self.Player`)) _output_get)
    (if (< _output_get 0.0)
      (`/Game/FirstPerson/Blueprints/BP_FirstPersonCharacter.Die` (`self.Player`)))))

(fn `OpenDoor`
  (returns (opened :type Boolean))
  (bind _player (`self.Player`))
  (if (not (`self.Opened`))
    (`GameplayStatics.PlaySound2D` "/Game/02_Sounds/Door-opening_modified.Door-opening_modified" 1.0 1.0 0.0 null null)
    (`self.OpenDoor_Animation`)
    (set `self.StartCountdown` true)
    (`/Game/FirstPerson/Player_UI.UpdateKeysCollected` (`/Game/FirstPerson/Blueprints/BP_FirstPersonCharacter.PlayerUI` _player) (`/Game/FirstPerson/Blueprints/BP_FirstPersonCharacter.KeysCollected` _player) (`/Game/FirstPerson/Blueprints/BP_FirstPersonCharacter.TotalNumOfKeys` _player))
    (`/Game/FirstPerson/Player_UI.ShowInfo` (`/Game/FirstPerson/Blueprints/BP_FirstPersonCharacter.PlayerUI` (`self.Player`)))
    (set `self.Opened` true)
    (return true)))

(fn `UserConstructionScript`
  (`parent.UserConstructionScript`))