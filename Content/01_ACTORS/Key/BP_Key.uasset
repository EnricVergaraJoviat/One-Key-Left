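; BP_Key is a key pickup that bobs up and down and gives the first-person character a key on overlap.
; Tick adds a sine-of-game-time Z offset to the root each frame without delta-time scaling.
; Box overlap calls AddKey on the character, plays a pickup sound, then destroys the actor after a short delay.
; DoOnce precedes the character cast, so the first overlap by any actor consumes it.
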(event `self.ReceiveTick`
  (params (DeltaSeconds :type "Float (single-precision)"))
  (`SceneComponent.K2_AddRelativeLocation` (`self.DefaultSceneRoot`) (`KismetMathLibrary.MakeVector` 0.0 0.0 (* (`KismetMathLibrary.Sin` (`KismetSystemLibrary.GetGameTimeInSeconds`)) 0.5)) false false))

(event `self.Box.OnComponentBeginOverlap`
  (params (OverlappedComponent :type "PrimitiveComponent Object Reference") (OtherActor :type "Actor Object Reference") (OtherComp :type "PrimitiveComponent Object Reference") (OtherBodyIndex :type Integer) (bFromSweep :type Boolean) (SweepResult :type "HitResult Structure (by ref)"))
  (`/Engine/EditorBlueprintResources/StandardMacros.DoOnce` false
    (:`Completed`
      (bind _asbp_first_person_character (cast `/Game/FirstPerson/Blueprints/BP_FirstPersonCharacter` OtherActor))
      (`/Game/FirstPerson/Blueprints/BP_FirstPersonCharacter.AddKey` _asbp_first_person_character)
      (`GameplayStatics.PlaySound2D` "/Game/02_Sounds/Hammer-Pickup.Hammer-Pickup" 1.0 1.0 0.0 null null)
      (`KismetSystemLibrary.Delay` 0.5)
      (`self.K2_DestroyActor`))))

(fn `UserConstructionScript`)