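; BP_FloorButton1 is a floor button that removes a wall and signals a door when the first-person player steps on it.
; It binds to the player's all-keys-collected event to turn its hieroglyph mesh green.
; Box overlap destroys SMWall13 regardless of keys, then calls OpenDoorMessage on Door through BPI_OpenDoor.
; If that returns true, the button's root drops down and its trigger and hieroglyph components are destroyed.
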(event `self.ReceiveBeginPlay`
  (bind _asbp_first_person_character (cast `/Game/FirstPerson/Blueprints/BP_FirstPersonCharacter` (`GameplayStatics.GetPlayerCharacter` 0)))
  (add `/Game/FirstPerson/Blueprints/BP_FirstPersonCharacter.AllKeysCollected` _asbp_first_person_character (delegate `AllKeysCollected`)))

(event `AllKeysCollected`
  (bind _sm_hieroglyph_008 (`self.SM_hieroglyph_008`))
  (if (`KismetSystemLibrary.IsValid` _sm_hieroglyph_008)
    (`PrimitiveComponent.SetMaterial` _sm_hieroglyph_008 0 "/Game/01_ACTORS/Floor_Button/emission_green.emission_green")))

(event `self.Box.OnComponentBeginOverlap`
  (params (OverlappedComponent :type "PrimitiveComponent Object Reference") (OtherActor :type "Actor Object Reference") (OtherComp :type "PrimitiveComponent Object Reference") (OtherBodyIndex :type Integer) (bFromSweep :type Boolean) (SweepResult :type "HitResult Structure (by ref)"))
  (bind _defaultsceneroot (`self.DefaultSceneRoot`))
  (bind _door (`self.Door`))
  (cast `/Game/FirstPerson/Blueprints/BP_FirstPersonCharacter` OtherActor)
  (set `self.ButtonPressed` true)
  (`self.K2_DestroyActor` (`self.SM_wall_13`))
  (`/Engine/EditorBlueprintResources/StandardMacros.IsValid` _door
    (:`Is Valid`
      (if (`KismetSystemLibrary.DoesImplementInterface` _door "/Game/01_ACTORS/Door/Logic/BPI_OpenDoor.BPI_OpenDoor_C")
        (bind _opened (message `/Game/01_ACTORS/Door/Logic/BPI_OpenDoor.OpenDoor` (`self.Door`)))
        (if _opened
          (`SceneComponent.K2_SetWorldLocation` _defaultsceneroot (+ (`SceneComponent.K2_GetComponentLocation` _defaultsceneroot) (0.0 0.0 -40.0)) false false)
          (`ActorComponent.K2_DestroyComponent` (`self.Box`))
          (`ActorComponent.K2_DestroyComponent` (`self.SM_hieroglyph_008`)))))))

(event `self.boto_apretar.OnComponentBeginOverlap`
  (params (OverlappedComponent :type "PrimitiveComponent Object Reference") (OtherActor :type "Actor Object Reference") (OtherComp :type "PrimitiveComponent Object Reference") (OtherBodyIndex :type Integer) (bFromSweep :type Boolean) (SweepResult :type "HitResult Structure (by ref)")))

(fn `UserConstructionScript`)